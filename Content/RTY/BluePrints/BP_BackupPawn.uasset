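; BP_BackupPawn is a pawn with keyboard shortcuts that trigger warp and alert states, apparently for testing.
; Keys 0 and 9 spawn the Earth and Badland warp actors at one hard-coded transform.
; Keys 7 and 8 set and clear AlertOn on the GI_Rty game instance cached at BeginPlay.
; An unconnected chain would move the VRPawn and show dialogue when EngineRoom is set, but never runs.
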(event `self.ReceiveBeginPlay`
  (bind _asgi_rty (cast `/Game/RTY/BluePrints/GI_Rty` (`GameplayStatics.GetGameInstance`)))
  (set `self.As GI Rty` _asgi_rty))

(event `Key|Zero`
  (params (Key :type "Key Structure"))
  (:`Pressed`
    (`|SpawnActorFromClass` "/Game/RTY/BluePrints/BP_WarpToEarth.BP_WarpToEarth_C" (`KismetMathLibrary.MakeTransform` (-20220.0 -303825.0 -6007.0) (struct :`Yaw` 90.0)) "Undefined" "MultiplyWithRoot" null null)))

(event `Key|Nine`
  (params (Key :type "Key Structure"))
  (:`Pressed`
    (`|SpawnActorFromClass` "/Game/RTY/BluePrints/BP_WarpToBadland.BP_WarpToBadland_C" (`KismetMathLibrary.MakeTransform` (-20220.0 -303825.0 -6007.0) (struct :`Yaw` 90.0)) "Undefined" "MultiplyWithRoot" null null)))

(event `Key|Seven`
  (params (Key :type "Key Structure"))
  (:`Pressed`
    (set `/Game/RTY/BluePrints/GI_Rty.bAlertOn` true (`self.As GI Rty`))))

(event `Key|Eight`
  (params (Key :type "Key Structure"))
  (:`Pressed`
    (set `/Game/RTY/BluePrints/GI_Rty.bAlertOn` false (`self.As GI Rty`))))

(fn `UserConstructionScript`)