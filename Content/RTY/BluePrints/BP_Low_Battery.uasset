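; BP_Low_Battery is a grabbable depleted battery that starts out at the battery socket.
; On BeginPlay it tints the energy core red, then moves itself to the first BP_BatterySocket found in the level with a fixed rotation and scale.
; Its GrabComponent events drive the core mesh: grabbing turns on physics simulation, and dropping turns the material color black.
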(event `self.ReceiveBeginPlay`
  (`MeshComponent.SetVectorParameterValueOnMaterials` (`self.SM_EnergyCore_A`) "Color" (1.0 0.0 0.0))
  (bind _outactors (`GameplayStatics.GetAllActorsOfClass` "/Game/RTY/BluePrints/BP_BatterySocket.BP_BatterySocket_C"))
  (bind _output_get (set `self.BP_BatterySocket` (`|GetArrayItem` _outactors)))
  (`self.K2_SetActorTransform` (`KismetMathLibrary.MakeTransform` (`self.K2_GetActorLocation` _output_get) (struct :`Pitch` 90.0) (2.0 2.0 2.0))))

(event `self.ReceiveTick`
  (params (DeltaSeconds :type "Float (single-precision)")))

(event `self.GrabComponent.OnGrabbed`
  (`PrimitiveComponent.SetSimulatePhysics` (`self.SM_EnergyCore_A`) true))

(event `self.GrabComponent.OnDropped`
  (`MeshComponent.SetVectorParameterValueOnMaterials` (`self.SM_EnergyCore_A`) "Color" (0.0 0.0 0.0)))

(fn `UserConstructionScript`)