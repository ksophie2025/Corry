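; Spline-based guide line actor that can be revealed in game through the ShowGuideLine event.
; The construction script adds an X-forward spline mesh component for each spline point, fitting it to that point and the next using local positions and tangents.
; The loop also runs on the last point, so its final segment requests an index past the end of the spline.
; ShowGuideLine only unhides the actor, with no logic here to hide it.
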(event `ShowGuideLine`
  (`self.SetActorHiddenInGame` false))

(fn `UserConstructionScript`
  (bind _spline (`self.Spline`))
  (bind _spline_2 (`self.Spline`))
  (for _index (range (`SplineComponent.GetNumberOfSplinePoints` (`self.Spline`)))
    (bind _returnvalue (`AddComponent|NODE_AddSplineMeshComponent-1`))
    (`SplineMeshComponent.SetForwardAxis` _returnvalue "X" true)
    (bind _returnvalue_2 (+ _index 1))
    (`SplineMeshComponent.SetStartAndEnd` _returnvalue (`SplineComponent.GetLocationAtSplinePoint` _spline_2 _index "Local") (`SplineComponent.GetTangentAtSplinePoint` _spline_2 _index "Local") (`SplineComponent.GetLocationAtSplinePoint` _spline _returnvalue_2 "Local") (`SplineComponent.GetTangentAtSplinePoint` _spline _returnvalue_2 "Local") true)))