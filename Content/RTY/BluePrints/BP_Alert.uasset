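; Alarm beacon actor that spins, flashes and sounds while the game instance's AlertOn flag is set.
; BeginPlay caches GI_Rty and spawns a persistent alarm sound; Tick polls the flag and calls AlamOn or AlamOff every frame.
; Chained timelines rotate two cubes 90 degrees apart and drive the point light and alarm material intensity.
; AlamOff stops the timelines, zeroes both intensities and mutes the sound via its volume multiplier.
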(event `AlamOn`
  (`AudioComponent.SetVolumeMultiplier` (`self.AlarmSound`) 0.01)
  (bind (_direction _0) (`Timeline|Timeline` :!label _label)
    (:`Update`
      (`SceneComponent.K2_SetRelativeRotation` (`self.Cube`) (`KismetMathLibrary.MakeRotator` 0.0 0.0 _0) false false)
      (`SceneComponent.K2_SetRelativeRotation` (`self.Cube1`) (`KismetMathLibrary.MakeRotator` 0.0 0.0 (+ _0 90.0)) false false)
      (bind (_direction_2 _newtrack_0) (`Timeline|Timeline_0` :!label _label_2)
        (:`Update`
          (`LightComponent.SetIntensity` (`self.PointLight`) _newtrack_0)
          (bind (_direction_3 _newtrack_0_2) (`Timeline|Timeline_1` :!label _label_3)
            (:`Update`
              (`MeshComponent.SetScalarParameterValueOnMaterials` (`self.SM_AlarmLight`) "Intensity" _newtrack_0_2))))))))

(event `AlamOff`
  (`|ExecutionSequence`
    (:`then_0`
      (goto _label :!via `Stop`))
    (:`then_1`
      (goto _label_2 :!via `Stop`))
    (:`then_2`
      (`LightComponent.SetIntensity` (`self.PointLight`) 0.0)
      (`MeshComponent.SetScalarParameterValueOnMaterials` (`self.SM_AlarmLight`) "Intensity" 0.0)
      (goto _label_3 :!via `Stop`))
    (:`then_3`
      (`AudioComponent.SetVolumeMultiplier` (`self.AlarmSound`) 0.0))))

(event `self.ReceiveBeginPlay`
  (bind _asgi_rty (cast `/Game/RTY/BluePrints/GI_Rty` (`GameplayStatics.GetGameInstance`)))
  (set `self.As GI Rty` _asgi_rty)
  (bind _returnvalue (`GameplayStatics.SpawnSoundAtLocation` "/Game/RTY/Sounds/Alarm.Alarm" (`self.K2_GetActorLocation`) (struct) 1.0 1.0 0.0 null null false))
  (set `self.AlarmSound` _returnvalue))

(event `self.ReceiveTick`
  (params (DeltaSeconds :type "Float (single-precision)"))
  (if (`/Game/RTY/BluePrints/GI_Rty.bAlertOn` (`self.As GI Rty`))
    (`self.AlamOn`)
    (else
      (`self.AlamOff`))))

(fn `UserConstructionScript`)