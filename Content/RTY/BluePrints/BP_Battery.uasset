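; BP_Battery is a battery Blueprint that changes the color of its energy core mesh over time.
; Tick adds delta seconds to a running timer and sets the Color material parameter on the mesh every frame.
; The core starts blue, turns white after a short interval, then stays red once the later threshold is reached, as nothing resets the timer.
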(event `self.ReceiveTick`
  (params (DeltaSeconds :type "Float (single-precision)"))
  (bind _output_get (set `self.CurrentTime` (+ DeltaSeconds (`self.CurrentTime`))))
  (if (<= _output_get 2.0)
    (`MeshComponent.SetVectorParameterValueOnMaterials` (`self.SM_EnergyCore_A`) "Color" (0.0 0.5 1.0))
    (elif (>= _output_get 5.0)
      (`MeshComponent.SetVectorParameterValueOnMaterials` (`self.SM_EnergyCore_A`) "Color" (1.0 0.0 0.1))
      (else
        (`MeshComponent.SetVectorParameterValueOnMaterials` (`self.SM_EnergyCore_A`) "Color" (1.0 1.0 1.0))))))

(fn `UserConstructionScript`)