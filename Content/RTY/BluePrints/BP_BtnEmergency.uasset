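; BP_BtnEmergency is a grabbable VR emergency power button whose single press randomly succeeds or fails to restart emergency power.
; On first grab, a coin flip selects the player pawn's dialogue and one of two timelines that move the button mesh along Z.
; Success spawns the emergency sound, while failure calls EmergencyFailed on the level's BP_Blackhole.
; Both of these calls run on every timeline update rather than once.
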(event `self.ReceiveBeginPlay`
  (bind _asvrpawn (cast `/Game/VRTemplate/Blueprints/VRPawn` (`GameplayStatics.GetPlayerCharacter` 0)))
  (set `self.As VRPawn` _asvrpawn)
  (bind _outactors (`GameplayStatics.GetAllActorsOfClass` "/Game/RTY/BluePrints/BP_Blackhole.BP_Blackhole_C"))
  (set `self.BlackHole` (`|GetArrayItem` _outactors)))

(event `self.GrabComponent.OnGrabbed`
  (bind _as_vrpawn (`self.As VRPawn`))
  (`/Engine/EditorBlueprintResources/StandardMacros.DoOnce` false
    (:`Completed`
      (if (`KismetMathLibrary.RandomBool`)
        (`/Game/VRTemplate/Blueprints/VRPawn.ShowDialogueAlpha` _as_vrpawn "15b-6" "26") ; 비상전원 가동 성공
        (bind (_direction _newtrack_0) (`Timeline|Timeline`)
          (:`Update`
            (`SceneComponent.K2_SetRelativeLocation` (`self.Merge_02AA5731`) (`KismetMathLibrary.MakeVector` 0.0 0.0 _newtrack_0) false false)
            (`GameplayStatics.SpawnSoundAtLocation` "/Game/RTY/Sounds/Emergency.Emergency" (`self.K2_GetActorLocation`) (struct) 1.0 1.0 0.0 null null)))
        (else
          (`/Game/VRTemplate/Blueprints/VRPawn.ShowDialogue` _as_vrpawn (`self.NewVar`)) ; 비상전원 재가동 실패
          (bind (_direction_2 _newtrack_0_2) (`Timeline|Timeline_0`)
            (:`Update`
              (`SceneComponent.K2_SetRelativeLocation` (`self.Merge_02AA5731`) (`KismetMathLibrary.MakeVector` 0.0 0.0 _newtrack_0_2) false false)
              ;[0 0 0] 태영이 블랙홀 이벤트
              (`/Game/RTY/BluePrints/BP_Blackhole.Emergency_Failed` (`self.BlackHole`)))))))))

(fn `UserConstructionScript`)