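; Black hole actor that homes in on the VR player's pawn with escalating sound and screen effects.
; On BeginPlay it caches the VRPawn, spawns a 2D sound and plays a timeline, which the Emergency_Failed event also plays.
; Timeline curves drive the sound volume, frame-time-scaled movement toward the player, actor scale, and post-process chromatic aberration and exposure.
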(event `self.ReceiveBeginPlay`
  (bind _asvrpawn (cast `/Game/VRTemplate/Blueprints/VRPawn` (`GameplayStatics.GetPlayerCharacter` 0)))
  (set `self.As VRPawn` _asvrpawn)
  (bind _returnvalue (`GameplayStatics.SpawnSound2D` "/Game/RTY/Sounds/BlackholeSound.BlackholeSound" 1.0 1.0 0.0 null false false))
  (bind (_direction _blackhole_move _postprocess_exposure _postprocess_chromaticaberration _scale _volume) (`Timeline|Timeline` :!label _label)
    (:`Update`
      (`AudioComponent.SetVolumeMultiplier` _returnvalue _volume)
      (`self.K2_SetActorLocation` (+ (`self.K2_GetActorLocation`) (* (`KismetMathLibrary.Normal` (- (`self.K2_GetActorLocation` (`self.As VRPawn`)) (`self.K2_GetActorLocation`)) 0.001) (* _blackhole_move (`GameplayStatics.GetWorldDeltaSeconds`)))))
      (bind _structout (setmembers `PostProcessSettings` :`StructRef` (make `PostProcessSettings` :`SceneFringeIntensity` _postprocess_chromaticaberration :`AutoExposureBias` _postprocess_exposure)))
      (set `PostProcessComponent.Settings` _structout (`self.PostProcess`))
      (`self.SetActorScale3D` (`KismetMathLibrary.Conv_DoubleToVector` _scale)))))

(event `Emergency_Failed`
  (goto _label))

(fn `UserConstructionScript`)