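; BP_ArcReacter is an animated arc reactor prop whose parts spin continuously on Tick.
; Reacter and Reacter1 roll at a constant delta-time-scaled rate, held at opposite 45-degree yaws.
; ArcPitch, ArcYaw and ArcRoll each turn on a separate axis at different multiples of RotationSpeed, which ramps up over time to a cap.
; These arc increments apply per frame without delta scaling, so their speed depends on frame rate.
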(event `self.ReceiveTick`
  (params (DeltaSeconds :type "Float (single-precision)"))
  (bind _returnvalue (* DeltaSeconds 50.0))
  (bind _main_roll (`KismetMathLibrary.BreakRotator` (`self.Main`)))
  (bind _main_0_roll (`KismetMathLibrary.BreakRotator` (`self.Main_0`)))
  (bind (_arc_roll _arc_pitch _arc_yaw) (`KismetMathLibrary.BreakRotator` (`self.Arc`)))
  (bind _output_get (set `self.Main` (`KismetMathLibrary.MakeRotator` (+ _returnvalue _main_roll) 0.0 45.0)))
  (`SceneComponent.K2_SetRelativeRotation` (`self.Reacter`) _output_get false false)
  (bind _output_get_2 (set `self.Main_0` (`KismetMathLibrary.MakeRotator` (+ _returnvalue _main_0_roll) 0.0 -45.0)))
  (`SceneComponent.K2_SetRelativeRotation` (`self.Reacter1`) _output_get_2 false false)
  (bind _output_get_3 (set `self.RotationSpeed` (+ (`self.RotationSpeed`) DeltaSeconds)))
  (`|ExecutionSequence`
    (:`then_0`
      (if (>= _output_get_3 8.0)
        (set `self.RotationSpeed` 8.0)))
    (:`then_1`
      (bind _output_get_4 (set `self.Arc` (`KismetMathLibrary.MakeRotator` (+ _output_get_3 _arc_roll) (+ (* _output_get_3 1.5) _arc_pitch) (+ (* _output_get_3 2.0) _arc_yaw))))
      (`SceneComponent.K2_SetRelativeRotation` (`self.Arc_Pitch`) (`KismetMathLibrary.MakeRotator` (.roll _output_get_4)) false false)
      (`SceneComponent.K2_SetRelativeRotation` (`self.Arc_Yaw`) (`KismetMathLibrary.MakeRotator` 0.0 (.pitch _output_get_4)) false false)
      (`SceneComponent.K2_SetRelativeRotation` (`self.Arc_Roll`) (`KismetMathLibrary.MakeRotator` 90.0 0.0 (.yaw _output_get_4)) false false))))

(fn `UserConstructionScript`)