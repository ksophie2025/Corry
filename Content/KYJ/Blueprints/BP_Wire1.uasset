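; BP_Wire1 is a wire-connection mission prop where a grabbed wire end is linked to a destination point.
; Destination overlap events set and clear a CanLink flag by matching "EndLoc" in the overlapping component's display name.
; When GrabComponent is dropped with CanLink true, EndLoc snaps to Destination's world location and MissionAlert's ClearColor material parameter turns blue to signal completion.
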(event `self.GrabComponent.OnDropped`
  (if (`self.bCanLink`)
    (`SceneComponent.K2_SetWorldLocation` (`self.EndLoc`) (`SceneComponent.K2_GetComponentLocation` (`self.destination`)) false false) ; 끝을 붙여라
    (`MeshComponent.SetVectorParameterValueOnMaterials` (`self.Mission_Alert`) "ClearColor" (0.0 0.5 1.0))))

(event `self.destination.OnComponentBeginOverlap`
  (params (OverlappedComponent :type "PrimitiveComponent Object Reference") (OtherActor :type "Actor Object Reference") (OtherComp :type "PrimitiveComponent Object Reference") (OtherBodyIndex :type Integer) (bFromSweep :type Boolean) (SweepResult :type "HitResult Structure (by ref)"))
  (if (`KismetStringLibrary.Contains` (`KismetSystemLibrary.GetDisplayName` OtherComp) "EndLoc")
    (set `self.bCanLink` true)))

(event `self.destination.OnComponentEndOverlap`
  (params (OverlappedComponent :type "PrimitiveComponent Object Reference") (OtherActor :type "Actor Object Reference") (OtherComp :type "PrimitiveComponent Object Reference") (OtherBodyIndex :type Integer))
  (if (`KismetStringLibrary.Contains` (`KismetSystemLibrary.GetDisplayName` OtherComp) "EndLoc")
    (set `self.bCanLink` false)))

(fn `UserConstructionScript`)