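; Engine room mission trigger for VR that plays a luck-dependent dialogue when the player grabs it.
; On grab, it reads the Lucky flag from GI_Rty and passes the lucky or unlucky start and break row names to ShowDialogueAlpha on the VRPawn.
; It then destroys itself, so the dialogue fires only once.
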(event `self.GrabComponent.OnGrabbed`
  (bind _asgi_rty (cast `/Game/RTY/BluePrints/GI_Rty` (`GameplayStatics.GetGameInstance`)))
  (if (`/Game/RTY/BluePrints/GI_Rty.bLucky` _asgi_rty)
    (bind _asvrpawn (cast `/Game/VRTemplate/Blueprints/VRPawn` (`GameplayStatics.GetPlayerPawn` 0)))
    (`/Game/VRTemplate/Blueprints/VRPawn.ShowDialogueAlpha` _asvrpawn (`self.StartRowName_Lucky`) (`self.BreakRowName_Lucky`))
    (`self.K2_DestroyActor`)
    (else
      (bind _asvrpawn_2 (cast `/Game/VRTemplate/Blueprints/VRPawn` (`GameplayStatics.GetPlayerPawn` 0)))
      (`/Game/VRTemplate/Blueprints/VRPawn.ShowDialogueAlpha` _asvrpawn_2 (`self.StartRowName_Unlucky`) (`self.BreakRowName_Unlucky`))
      (`self.K2_DestroyActor`))))

(fn `UserConstructionScript`)