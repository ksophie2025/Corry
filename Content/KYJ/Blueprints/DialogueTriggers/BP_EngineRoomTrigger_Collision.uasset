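; A one-shot collision trigger, named for the engine room, that shows branching dialogue when the player's VRPawn overlaps its box.
; It reads the Lucky flag on the GI_Rty game instance, which reflects an earlier dialogue choice, to pick the lucky or unlucky start and break row names.
; It passes those rows to the pawn's ShowDialogueAlpha, then destroys itself.
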(event `self.Box.OnComponentBeginOverlap`
  (params (OverlappedComponent :type "PrimitiveComponent Object Reference") (OtherActor :type "Actor Object Reference") (OtherComp :type "PrimitiveComponent Object Reference") (OtherBodyIndex :type Integer) (bFromSweep :type Boolean) (SweepResult :type "HitResult Structure (by ref)"))
  (bind _asvrpawn (cast `/Game/VRTemplate/Blueprints/VRPawn` OtherActor)) ; 부딪힌 게 플레이어니?
  (set `self.As VRPawn` _asvrpawn)
  (bind _asgi_rty (cast `/Game/RTY/BluePrints/GI_Rty` (`GameplayStatics.GetGameInstance`)))
  (if (`/Game/RTY/BluePrints/GI_Rty.bLucky` _asgi_rty)
    (`/Game/VRTemplate/Blueprints/VRPawn.ShowDialogueAlpha` (`self.As VRPawn`) (`self.Start Row Name Lucky`) (`self.Break Row Name Lucky`))
    (`self.K2_DestroyActor`)
    (else
      (`/Game/VRTemplate/Blueprints/VRPawn.ShowDialogueAlpha` (`self.As VRPawn`) (`self.Start Row Name Unlucky`) (`self.Break Row Name Unlucky`))
      (`self.K2_DestroyActor`))))

(fn `UserConstructionScript`)