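; BP_bean is a grabbable coffee bean actor that works with BP_CoffeeMachine.
; Tick searches for all coffee machines every frame, and the drop handler reads BeanFilled on the first one found.
; When dropped, the actor destroys itself if that flag is true; otherwise the Bean component snaps back to the scene root's location and rotation.
; An unconnected node that would clear BeanFilled never runs.
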(event `self.ReceiveTick`
  (params (DeltaSeconds :type "Float (single-precision)"))
  (bind _outactors (`GameplayStatics.GetAllActorsOfClass` "/Game/KSH/Blueprints/BP_CoffeeMachine.BP_CoffeeMachine_C")))

(event `self.GrabComponent.OnDropped`
  (bind _defaultsceneroot (`self.DefaultSceneRoot`))
  (if (`/Game/KSH/Blueprints/BP_CoffeeMachine.bBeanFilled` (`|GetArrayItem` (stale `self.ReceiveTick` _outactors)))
    (`self.K2_DestroyActor`)
    (else
      (`SceneComponent.K2_SetWorldLocationAndRotation` (`self.Bean`) (`SceneComponent.K2_GetComponentLocation` _defaultsceneroot) (`SceneComponent.K2_GetComponentRotation` _defaultsceneroot) false false))))

(fn `UserConstructionScript`)