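; BP_CoffeeMachine is a coffee machine with a grabbable pot (Kanne) that brews when a bean actor is added.
; A BP_bean overlapping Vann sets BeanFilled and toggles the bean visual, then after a short delay toggles the coffee water visual and sets CoffeeReady.
; Dropping the grab component snaps Kanne back to the root's transform, gated by Holdingkanne, which is set on grab and never cleared here.
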(event `self.GrabComponent.OnGrabbed`
  (set `self.bHoldingkanne` true))

(event `self.GrabComponent.OnDropped`
  (bind _defaultsceneroot (`self.DefaultSceneRoot`))
  (if (`self.bHoldingkanne`)
    (`SceneComponent.K2_SetWorldLocationAndRotation` (`self.Kanne`) (`SceneComponent.K2_GetComponentLocation` _defaultsceneroot) (`SceneComponent.K2_GetComponentRotation` _defaultsceneroot) false false)))

(event `self.Vann.OnComponentBeginOverlap`
  (params (OverlappedComponent :type "PrimitiveComponent Object Reference") (OtherActor :type "Actor Object Reference") (OtherComp :type "PrimitiveComponent Object Reference") (OtherBodyIndex :type Integer) (bFromSweep :type Boolean) (SweepResult :type "HitResult Structure (by ref)"))
  (cast `/Game/KSH/Blueprints/BP_bean` OtherActor)
  (set `self.bBeanFilled` true)
  (`SceneComponent.ToggleVisibility` (`self.coffee bean`) false)
  (`KismetSystemLibrary.Delay` 1.7)
  (`SceneComponent.ToggleVisibility` (`self.coffe water`) false)
  (set `self.bCoffeeReady` true))

(event `self.Kanne.OnComponentBeginOverlap`
  (params (OverlappedComponent :type "PrimitiveComponent Object Reference") (OtherActor :type "Actor Object Reference") (OtherComp :type "PrimitiveComponent Object Reference") (OtherBodyIndex :type Integer) (bFromSweep :type Boolean) (SweepResult :type "HitResult Structure (by ref)")))

(fn `UserConstructionScript`)