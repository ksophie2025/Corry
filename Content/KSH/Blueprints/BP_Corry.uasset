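; BP_Corry is an actor built from a MetaHuman face mesh, a cone and a static mesh that bobs and changes appearance with the player's score.
; Tick drives its relative Z from a sine of accumulated time and enables custom depth on all three meshes for outlining.
; It also reads Score from GI_Rty every frame, switching overlay material and stencil value at a fixed threshold.
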(event `self.ReceiveTick`
  (params (DeltaSeconds :type "Float (single-precision)"))
  (bind _newmetahumanidentity_facemesh (`self.NewMetaHumanIdentity_FaceMesh`))
  (bind _newmetahumanidentity_facemesh_2 (`self.NewMetaHumanIdentity_FaceMesh`))
  (`|ExecutionSequence`
    (:`then_0`
      (bind _output_get (set `self.NewVar` (+ DeltaSeconds (`self.NewVar`))))
      (`self.K2_SetActorRelativeLocation` (`KismetMathLibrary.MakeVector` 0.0 0.0 (* (`KismetMathLibrary.DegSin` (* _output_get 100.0)) 1.5))))
    (:`then_1`
      ;[1 1 1] outline
      (`PrimitiveComponent.SetCustomDepthStencilValue` _newmetahumanidentity_facemesh_2 (`self.Stencil Val`))
      (`PrimitiveComponent.SetCustomDepthStencilValue` (`self.Cone`) (`self.Stencil Val`))
      (`PrimitiveComponent.SetCustomDepthStencilValue` (`self.StaticMesh`) (`self.Stencil Val`))
      (`PrimitiveComponent.SetRenderCustomDepth` _newmetahumanidentity_facemesh_2 true)
      (`PrimitiveComponent.SetRenderCustomDepth` (`self.Cone`) true)
      (`PrimitiveComponent.SetRenderCustomDepth` (`self.StaticMesh`) true))
    (:`then_2`
      (bind _asgi_rty (cast `/Game/RTY/BluePrints/GI_Rty` (`GameplayStatics.GetGameInstance`)))
      (if (> (`/Game/RTY/BluePrints/GI_Rty.Score` _asgi_rty) 24)
        ;[0 0.762 1] Comment
        (`MeshComponent.SetOverlayMaterial` _newmetahumanidentity_facemesh "/Game/KSH/Materials/outline/M_ooo.M_ooo")
        (`MeshComponent.SetOverlayMaterial` (`self.Cone`) "/Game/KSH/Materials/outline/M_ooo.M_ooo")
        (`MeshComponent.SetOverlayMaterial` (`self.StaticMesh`) "/Game/KSH/Materials/outline/M_ooo.M_ooo")
        (set `self.Stencil Val` 1)
        (else
          ;[1 0.343 0.3729] Comment
          (`MeshComponent.SetOverlayMaterial` _newmetahumanidentity_facemesh "/Game/KSH/Materials/outline/M_ooo1.M_ooo1")
          (`MeshComponent.SetOverlayMaterial` (`self.Cone`) "/Game/KSH/Materials/outline/M_ooo1.M_ooo1")
          (`MeshComponent.SetOverlayMaterial` (`self.StaticMesh`) "/Game/KSH/Materials/outline/M_ooo1.M_ooo1")
          (set `self.Stencil Val` 2))))))

(fn `UserConstructionScript`)