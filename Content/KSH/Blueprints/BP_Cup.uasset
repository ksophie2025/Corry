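; BP_Cup is a cup actor that reacts to overlapping a coffee machine.
; When its Cup component begins overlapping a BP_CoffeeMachine whose CoffeeReady is set, it toggles the visibility of CupCoffeeWater.
; Debug prints show the overlap participants and cast failures, and the node setting CoffeeFill is left disconnected.
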(event `self.cup.OnComponentBeginOverlap`
  (params (OverlappedComponent :type "PrimitiveComponent Object Reference") (OtherActor :type "Actor Object Reference") (OtherComp :type "PrimitiveComponent Object Reference") (OtherBodyIndex :type Integer) (bFromSweep :type Boolean) (SweepResult :type "HitResult Structure (by ref)"))
  (`KismetSystemLibrary.PrintString` (`KismetSystemLibrary.GetDisplayName` OverlappedComponent) true true (struct :`G` 0.070476 :`B` 1.0 :`A` 1.0) 50.0)
  (`KismetSystemLibrary.PrintString` (`KismetSystemLibrary.GetDisplayName` OtherActor) true true (struct :`R` 1.0 :`B` 0.174332 :`A` 1.0) 50.0)
  (`KismetSystemLibrary.PrintString` (`KismetSystemLibrary.GetDisplayName` OtherComp) true true (struct :`G` 1.0 :`B` 0.115952 :`A` 1.0) 50.0)
  (bind _asbp_coffee_machine (cast `/Game/KSH/Blueprints/BP_CoffeeMachine` OtherActor)
    (:`then`
      (`KismetSystemLibrary.PrintString` "overlap")
      (if (`/Game/KSH/Blueprints/BP_CoffeeMachine.bCoffeeReady` _asbp_coffee_machine)
        (`SceneComponent.ToggleVisibility` (`self.cup coffee water`) false)))
    (:`CastFailed`
      (`KismetSystemLibrary.PrintString` "Cast failed!!!!!!!!!coffe machine!!!!!!!!!!!!!!!!!!" true true (struct :`R` 1.0 :`G` 0.043376 :`A` 1.0) 50.0))))

(fn `UserConstructionScript`)